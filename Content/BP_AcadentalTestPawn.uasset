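; Test pawn for manipulating scene objects with the mouse and logging each action to a file.
; Left-click picks an actor and drags it via a physics or normal transform, right-drag rotates it, and the wheel scales it.
; Tick polls held buttons, with rotation taking priority, while button releases and wheel steps log the HitActor's resulting transform.
; It also creates the HUD on BeginPlay and opens a single logout confirmation widget on Tab.
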(event `self.ReceiveBeginPlay`
  (bind _returnvalue (`|CreateWidget` "/Game/Widgets/WBP_HUD.WBP_HUD_C"))
  (`UserWidget.AddToViewport` _returnvalue 0))

(event `self.ReceiveTick`
  (params (DeltaSeconds :type "Float (single-precision)"))
  (bind _returnvalue (`GameplayStatics.GetPlayerController` 0))
  (if (`PlayerController.IsInputKeyDown` _returnvalue "RightMouseButton")
    (`self.Rotate`)
    (elif (`PlayerController.IsInputKeyDown` _returnvalue "LeftMouseButton")
      (if (`self.SimulatingPhysics`)
        (`self.PhysicsTransform`)
        (else
          (`self.NormalTransform`))))))

(event `Key|LeftMouseButton`
  (params (Key :type "Key Structure"))
  (:`Pressed`
    (`self.GetManipulateActor`))
  (:`Released`
    (bind _hitactor (`self.HitActor`)
      (:`then`
        (`self.LogActionToFile` "Transform" (`KismetSystemLibrary.GetObjectName` _hitactor) (`KismetStringLibrary.Conv_VectorToString` (`self.K2_GetActorLocation` _hitactor))))
      (:`else`))))

(event `Key|RightMouseButton`
  (params (Key :type "Key Structure"))
  (bind (_returnvalue_roll _returnvalue_pitch _returnvalue_yaw) (`KismetMathLibrary.BreakRotator` (`SceneComponent.K2_GetComponentRotation` (`self.Camera`))))
  (:`Pressed`
    (`self.RotateSetActor` _returnvalue_yaw))
  (:`Released`
    (bind _hitactor (`self.HitActor`)
      (:`then`
        (`self.LogActionToFile` "Rotate" (`KismetSystemLibrary.GetObjectName` _hitactor) (`KismetStringLibrary.Conv_RotatorToString` (`self.K2_GetActorRotation` _hitactor))))
      (:`else`))))

(event `Key|MouseScrollUp`
  (params (Key :type "Key Structure"))
  (:`Pressed`
    (`self.Scale` (`self.ScaleDelta`))
    (bind _hitactor (`self.HitActor` :!label _label)
      (:`then`
        (`self.LogActionToFile` "Scale" (`KismetSystemLibrary.GetObjectName` _hitactor) (`KismetStringLibrary.Conv_VectorToString` (`self.GetActorScale3D` _hitactor))))
      (:`else`))))

(event `Key|MouseScrollDown`
  (params (Key :type "Key Structure"))
  (:`Pressed`
    (`self.Scale` (* (`self.ScaleDelta`) -1.0))
    (goto _label)))

(event `Key|Tab`
  (params (Key :type "Key Structure"))
  (:`Pressed`
    (`self.OpenLogoutScreen`)))

(fn `OpenLogoutScreen`
  (`self.LogoutWidget`
    (:`then`)
    (:`else`
      (bind _returnvalue (`|CreateWidget` "/Game/Widgets/WBP_LogoutConfirmation.WBP_LogoutConfirmation_C"))
      (bind _output_get (set `self.LogoutWidget` _returnvalue))
      (`UserWidget.AddToViewport` _output_get 0))))

(fn `UserConstructionScript`)